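; BP_Win is a win trigger actor that ends play with a victory screen when something overlaps it.
; On overlap it casts the player pawn to PhysicsBallBP rather than checking the overlapping actor, then plays the win music and increments the ball's Score.
; It then switches to UI-only input with a visible, locked cursor and replaces all existing widgets with the UI_Win widget.
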(event Collision|EventActorBeginOverlap
  (params (OtherActor :type Actor%20Object%20Reference))
  (bind _returnvalue (Game|GetPlayerController 0))
  (Utilities|IsValid "/Game/RollingBP/Blueprints/PhysicsBallBP.PhysicsBallBP"
    (:Is%20Valid
      (Utilities|Casting|CastToPhysicsBallBP (Game|Player|GetPlayerPawn 0))
      (Audio|PlaySound2D "/Game/Audio/BGM/BGMWin.BGMWin" 1.0 1.0 0.0 0 0)
      (bind _asphysics_ball_bp (Utilities|Casting|CastToPhysicsBallBP (Game|Player|GetPlayerPawn 0)))
      (bind _result (Math|Integer|IncrementInt (Variables|/Game/RollingBP/Blueprints/PhysicsBallBP.PhysicsBallBP_C|GetScore _asphysics_ball_bp))
        (:%20%20
          (Variables|/Game/RollingBP/Blueprints/PhysicsBallBP.PhysicsBallBP_C|SetScore _asphysics_ball_bp _result)
          (Input|SetInputModeUIOnly _returnvalue 0 "LockAlways")
          (Variables|/Script/Engine.PlayerController|SetbShowMouseCursor _returnvalue true)
          (Viewport|RemoveAllWidgets)
          (bind _returnvalue_2 (UserInterface|CreateWidget "/Game/UI/UI_Win.UI_Win_C" _returnvalue))
          (UserInterface|Viewport|AddtoViewport _returnvalue_2 0))))))

(fn ConstructionScript)