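; Death hole for a rolling-ball game that costs the player a life or ends the game on overlap.
; On overlap, it checks a ball reference, plays the game-over sound and casts the player pawn to PhysicsBallBP.
; With lives to spare, it decrements Lives, briefly delays, then moves the ball to RestartPosition and resets its physics velocities.
; On the last life, it pauses, switches to UI-only input with a cursor and replaces all widgets with UI_GameOver.
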(event Collision|EventActorBeginOverlap
  (params (OtherActor :type Actor%20Object%20Reference))
  (bind _returnvalue (Game|GetPlayerController 0))
  ;[1 1 1] Trigger Death Restart new player
  (Utilities|IsValid "/Game/RollingBP/Blueprints/PhysicsBallBP.PhysicsBallBP"
    (:Is%20Valid
      (Audio|PlaySound2D "/Game/Audio/BGM/BGMGameOver.BGMGameOver" 1.0 1.0 0.0 0 0)
      (bind _asphysics_ball_bp (Utilities|Casting|CastToPhysicsBallBP (Game|Player|GetPlayerPawn 0)))
      (Math|Integer|CompareInt (- (Variables|/Game/RollingBP/Blueprints/PhysicsBallBP.PhysicsBallBP_C|GetLives _asphysics_ball_bp) 1) 1
        (:>
          (bind _result (Math|Integer|DecrementInt (Variables|/Game/RollingBP/Blueprints/PhysicsBallBP.PhysicsBallBP_C|GetLives _asphysics_ball_bp) :!label _label)
            (:%20%20
              (Variables|/Game/RollingBP/Blueprints/PhysicsBallBP.PhysicsBallBP_C|SetLives _asphysics_ball_bp _result)
              (Utilities|FlowControl|Delay 0.2)
              (Transformation|SetActorLocation _asphysics_ball_bp (Variables|Default|GetRestart%20Position) false false)
              (Class|PrimitiveComponent|SetAllPhysicsLinearVelocity (Variables|/Game/RollingBP/Blueprints/PhysicsBallBP.PhysicsBallBP_C|GetBall _asphysics_ball_bp) "0, 0, 0" false)
              (Class|PrimitiveComponent|SetAllPhysicsAngularVelocityinDegrees (Variables|/Game/RollingBP/Blueprints/PhysicsBallBP.PhysicsBallBP_C|GetBall _asphysics_ball_bp) (Variables|Default|GetRestart%20Velocity) false))))
        (:==
          (goto _label))
        (:<
          ;[1 1 1] Trigger Game Over
          (Game|SetGamePaused true)
          (Input|SetInputModeUIOnly _returnvalue 0 "LockAlways")
          (Variables|/Script/Engine.PlayerController|SetbShowMouseCursor _returnvalue true)
          (Viewport|RemoveAllWidgets)
          (bind _returnvalue_2 (UserInterface|CreateWidget "/Game/UI/UI_GameOver.UI_GameOver_C"))
          (UserInterface|Viewport|AddtoViewport _returnvalue_2 0))))))

(fn ConstructionScript)